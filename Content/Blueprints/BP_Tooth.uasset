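; Carryable tooth pickup that buffs the first-person character who touches it, reveals spell and frame UI, and triggers a chest spawn.
; A timeline offsets the mesh vertically while Tick spins it and snaps the actor to the carrier's ToothPoint.
; Drop functions relaunch it via ProjectileMovement, randomly upward or from the player's drop point, and destroy the BP_ChestTeeth.
; Only the voluntary drop ends the buff here.
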(event Custom|VoluntaryDropEvent)

(event EventBeginPlay
  (bind _returnvalue (Actor|GetActorOfClass "/Game/Blueprints/BP_ChestSpanwer.BP_ChestSpanwer_C"))
  (Variables|Default|SetRefChestSpawner _returnvalue)
  (bind _alpha_track (Timeline|Timeline PlayFromStart)
    (:Update
      (Transformation|SetRelativeLocation (Variables|Default|GetToothMesh) (Math|Vector|Lerp(Vector) "0, 0, 0" "0.000000,0.000000,10.000000" _alpha_track) false false))))

(event EventTick
  (params (DeltaSeconds :type Float%20%28single-precision%29))
  (Utilities|FlowControl|Sequence
    (:then_0
      (if (Variables|Default|GetIsTake)
        (Transformation|SetActorLocation (Transformation|GetWorldLocation (Variables|/Game/FirstPerson/Blueprints/BP_FirstPersonCharacter.BP_FirstPersonCharacter_C|GetToothPoint (Variables|Default|GetPlayer))) false false)))
    (:then_1
      (Transformation|AddLocalRotation (Variables|Default|GetToothMesh) "0.000000,2.000000,0.000000" false false))))

(event Collision|EventActorBeginOverlap
  (params (OtherActor :type Actor%20Object%20Reference))
  (bind _projectilemovement (Variables|Default|GetProjectileMovement))
  (if (not (Variables|Default|GetIsTake))
    (bind _asbp_first_person_character (Utilities|Casting|CastToBP_FirstPersonCharacter OtherActor))
    (Variables|Default|SetPlayer _asbp_first_person_character)
    (Variables|/Game/FirstPerson/Blueprints/BP_FirstPersonCharacter.BP_FirstPersonCharacter_C|SetHaveTooth _asbp_first_person_character true)
    (Default|OnToothBuff _asbp_first_person_character)
    (Widget|SetVisibility (Variables|/Game/Blueprints/Widget/WB_Spell.WB_Spell_C|GetSpell_UI_Dash (Variables|/Game/FirstPerson/Blueprints/BP_FirstPersonCharacter.BP_FirstPersonCharacter_C|GetRef_UI_Spell _asbp_first_person_character)) "Visible")
    (Widget|SetVisibility (Variables|/Game/Blueprints/Widget/WB_Cadre.WB_Cadre_C|GetCadreOr (Variables|/Game/FirstPerson/Blueprints/BP_FirstPersonCharacter.BP_FirstPersonCharacter_C|GetRef_UI_Cadre _asbp_first_person_character)) "Visible")
    (Variables|/Game/FirstPerson/Blueprints/BP_FirstPersonCharacter.BP_FirstPersonCharacter_C|SetTooth _asbp_first_person_character self)
    (Default|NumberOfWing (Variables|/Game/FirstPerson/Blueprints/BP_FirstPersonCharacter.BP_FirstPersonCharacter_C|GetRef_UI_Wing _asbp_first_person_character))
    (Variables|Default|SetIsTake true)
    (Default|SpawnChest (Variables|Default|GetRefChestSpawner))
    (Game|Components|ProjectileMovement|SetVelocityinLocalSpace _projectilemovement "0, 0, 0")
    (Variables|/Script/Engine.ProjectileMovementComponent|SetProjectileGravityScale _projectilemovement 0.0)))

(fn ConstructionScript)

(fn Drop
  (bind _projectilemovement (Variables|Default|GetProjectileMovement))
  (Variables|Default|SetIsTake false)
  (Components|Movement|SetUpdatedComponent _projectilemovement (Variables|Default|GetBox))
  (Game|Components|ProjectileMovement|SetVelocityinLocalSpace _projectilemovement (* (Math|Random|RandomUnitVectorinConeinDegrees "0.000000,0.000000,1.000000" 9e+01) 5e+02))
  (Components|Activation|Activate _projectilemovement true)
  (Variables|/Script/Engine.ProjectileMovementComponent|SetProjectileGravityScale _projectilemovement 1.0)
  (bind _returnvalue (Actor|GetActorOfClass "/Game/Blueprints/BP_ChestTeeth.BP_ChestTeeth_C"))
  (Actor|DestroyActor _returnvalue))

(fn VoluntaryDrop
  (bind _projectilemovement (Variables|Default|GetProjectileMovement))
  (bind _player (Variables|Default|GetPlayer))
  (bind _toothdropspawn (Variables|/Game/FirstPerson/Blueprints/BP_FirstPersonCharacter.BP_FirstPersonCharacter_C|GetToothDropSpawn _player))
  (Variables|Default|SetIsTake false)
  (Transformation|SetActorLocationAndRotation (Transformation|GetWorldLocation _toothdropspawn) (Transformation|GetWorldRotation _toothdropspawn))
  (Components|Movement|SetUpdatedComponent _projectilemovement (Variables|Default|GetBox))
  (Game|Components|ProjectileMovement|SetVelocityinLocalSpace _projectilemovement (* (Math|Vector|GetForwardVector _toothdropspawn) 2.5e+02))
  (Components|Activation|Activate _projectilemovement true)
  (Variables|/Script/Engine.ProjectileMovementComponent|SetProjectileGravityScale _projectilemovement 1.0)
  (bind _returnvalue (Actor|GetActorOfClass "/Game/Blueprints/BP_ChestTeeth.BP_ChestTeeth_C"))
  (Actor|DestroyActor _returnvalue)
  (Default|OnEndToothBuff (Variables|Default|GetPlayer)))