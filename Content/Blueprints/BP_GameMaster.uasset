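; BP_GameMaster spawns the local multiplayer players at level start, one per PlayerStart in the level.
; For each start point it creates a local player, using the loop index as the player ID.
; It then spawns a BP_FirstPersonCharacter at that transform, stores the ID on it, and adds IMC_Default to that player's Enhanced Input subsystem.
; The matching controller, newly created or fetched by index for existing players, possesses the character.
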(event EventBeginPlay
  (bind _returnvalue (Game|GetPlayerController 0))
  ;[0.15 0.15 0.15 0.5 74] Système de spawn des joueurs / Création d'une liste des joueurs
  ;;[0.8385 0.8385 0.8385 0.5] Récupérer la position et l'index des joueurs 1 par 1
  (bind _outactors (Actor|GetAllActorsOfClass "/Script/Engine.PlayerStart"))
  (for (_array_element _array_index) _outactors
    (bind _output_get (Variables|Default|SetPlayer%20ID _array_index))
    (Variables|Default|SetSpawn%20Transform (Transformation|GetActorTransform _array_element))
    (bind _returnvalue_2 (Class|GameplayStatics|CreatePlayer _output_get))
    (bind _output_get_2 (Variables|Default|SetRef%20Controller _returnvalue_2))
    (if (> (Variables|Default|GetPlayer%20ID) 0)
      (Utilities|IsValid _output_get_2
        (:Is%20Valid
          ;;[0.4348 0.09284 0.09284 0.5] Pour les autres joueurs
          (Input|AddMappingContext (PlayerController|LocalPlayerSubsystems|GetEnhancedInputLocalPlayerSubsystem _output_get_2) "/Game/Input/IMC_Default.IMC_Default" (Variables|Default|GetPlayer%20ID) "(bIgnoreAllPressedKeysUntilRelease=True,bForceImmediately=False,bNotifyUserSettings=False)")
          (bind _returnvalue_3 (Game|SpawnActorfromClass "/Game/FirstPerson/Blueprints/BP_FirstPersonCharacter.BP_FirstPersonCharacter_C" (Variables|Default|GetSpawn%20Transform) "Undefined" "MultiplyWithRoot" 0 0 0))
          (Variables|/Game/FirstPerson/Blueprints/BP_FirstPersonCharacter.BP_FirstPersonCharacter_C|SetIdPlayer _returnvalue_3 (Variables|Default|GetPlayer%20ID))
          (Pawn|Possess _output_get_2 _returnvalue_3))
        (:Is%20Not%20Valid
          ;;[0.05217 0.7292 0.2087 0.5] Si le Controller existe déjà
          (Input|AddMappingContext (PlayerController|LocalPlayerSubsystems|GetEnhancedInputLocalPlayerSubsystem (Game|GetPlayerController (Variables|Default|GetPlayer%20ID))) "/Game/Input/IMC_Default.IMC_Default" (Variables|Default|GetPlayer%20ID) "(bIgnoreAllPressedKeysUntilRelease=True,bForceImmediately=False,bNotifyUserSettings=False)")
          (bind _returnvalue_4 (Game|SpawnActorfromClass "/Game/FirstPerson/Blueprints/BP_FirstPersonCharacter.BP_FirstPersonCharacter_C" (Variables|Default|GetSpawn%20Transform) "Undefined" "MultiplyWithRoot" 0 0 0))
          (Variables|/Game/FirstPerson/Blueprints/BP_FirstPersonCharacter.BP_FirstPersonCharacter_C|SetIdPlayer _returnvalue_4 (Variables|Default|GetPlayer%20ID))
          (Pawn|Possess (Game|GetPlayerController (Variables|Default|GetPlayer%20ID)) _returnvalue_4)))
      (else
        ;;[0.07724 0.196 0.8177 0.5] Pour le joueur 1
        (Input|AddMappingContext (PlayerController|LocalPlayerSubsystems|GetEnhancedInputLocalPlayerSubsystem _returnvalue) "/Game/Input/IMC_Default.IMC_Default" 0 "(bIgnoreAllPressedKeysUntilRelease=True,bForceImmediately=False,bNotifyUserSettings=False)")
        (bind _returnvalue_5 (Game|SpawnActorfromClass "/Game/FirstPerson/Blueprints/BP_FirstPersonCharacter.BP_FirstPersonCharacter_C" (Variables|Default|GetSpawn%20Transform) "Undefined" "MultiplyWithRoot" 0 0 0))
        (bind _output_get_3 (Variables|/Game/FirstPerson/Blueprints/BP_FirstPersonCharacter.BP_FirstPersonCharacter_C|SetIdPlayer _returnvalue_5 (Variables|Default|GetPlayer%20ID)))
        (Development|PrintString (Utilities|String|ToString(Integer) _output_get_3) true true "(R=1.000000,G=0.047280,B=0.000000,A=1.000000)" 1e+01)
        (Pawn|Possess _returnvalue _returnvalue_5)))))

(fn ConstructionScript)