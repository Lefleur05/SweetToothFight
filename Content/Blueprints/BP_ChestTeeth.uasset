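; BP_ChestTeeth is a single-use deposit point where the first-person character banks a carried tooth for a point.
; On overlap with a character holding a tooth, it increments the score, clears the carry state and ends the tooth buff.
; It then updates the score and wing widgets, hides the dash and gold frame UI, and destroys the carried tooth.
; Finally it tells the BP_ToothSpawner to spawn another tooth and destroys itself.
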(event Collision|EventActorBeginOverlap
  (params (OtherActor :type Actor%20Object%20Reference))
  (bind _asbp_first_person_character (Utilities|Casting|CastToBP_FirstPersonCharacter OtherActor))
  (if (Variables|/Game/FirstPerson/Blueprints/BP_FirstPersonCharacter.BP_FirstPersonCharacter_C|GetHaveTooth _asbp_first_person_character)
    (Variables|/Game/FirstPerson/Blueprints/BP_FirstPersonCharacter.BP_FirstPersonCharacter_C|SetCountPoint _asbp_first_person_character (+ (Variables|/Game/FirstPerson/Blueprints/BP_FirstPersonCharacter.BP_FirstPersonCharacter_C|GetCountPoint _asbp_first_person_character) 1))
    (Variables|/Game/FirstPerson/Blueprints/BP_FirstPersonCharacter.BP_FirstPersonCharacter_C|SetHaveTooth _asbp_first_person_character false)
    (Default|OnEndToothBuff _asbp_first_person_character)
    (Default|FillTooth (Variables|/Game/FirstPerson/Blueprints/BP_FirstPersonCharacter.BP_FirstPersonCharacter_C|GetRef_UI_Score _asbp_first_person_character))
    (Widget|SetVisibility (Variables|/Game/Blueprints/Widget/WB_Spell.WB_Spell_C|GetSpell_UI_Dash (Variables|/Game/FirstPerson/Blueprints/BP_FirstPersonCharacter.BP_FirstPersonCharacter_C|GetRef_UI_Spell _asbp_first_person_character)) "Hidden")
    (Widget|SetVisibility (Variables|/Game/Blueprints/Widget/WB_Cadre.WB_Cadre_C|GetCadreOr (Variables|/Game/FirstPerson/Blueprints/BP_FirstPersonCharacter.BP_FirstPersonCharacter_C|GetRef_UI_Cadre _asbp_first_person_character)) "Hidden")
    (Default|NumberOfWing (Variables|/Game/FirstPerson/Blueprints/BP_FirstPersonCharacter.BP_FirstPersonCharacter_C|GetRef_UI_Wing _asbp_first_person_character))
    (Utilities|IsValid (Variables|/Game/FirstPerson/Blueprints/BP_FirstPersonCharacter.BP_FirstPersonCharacter_C|GetTooth _asbp_first_person_character)
      (:Is%20Valid
        (Actor|DestroyActor (Variables|/Game/FirstPerson/Blueprints/BP_FirstPersonCharacter.BP_FirstPersonCharacter_C|GetTooth _asbp_first_person_character)))
      (:Is%20Not%20Valid
        _))
    (bind _returnvalue (Actor|GetActorOfClass "/Game/Blueprints/BP_ToothSpawner.BP_ToothSpawner_C"))
    (Default|SpawnTooth _returnvalue)
    (Actor|DestroyActor)))

(fn ConstructionScript)