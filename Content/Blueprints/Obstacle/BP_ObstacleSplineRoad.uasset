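; BP_ObstacleSplineRoad is an obstacle actor that travels along the spline of a referenced SplineRoad.
; The construction script applies the configurable mesh.
; On BeginPlay, a timeline with its play rate scaled by TimeToEndPath drives an alpha over the spline's length.
; Each update sets the actor's world location and rotation from that distance along the spline.
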(event Custom|FollowSpline
  (bind _splineroad (Variables|Default|GetSplineRoad))
  (bind _spline (Variables|/Game/Blueprints/SplineMesh/SplineRoad.SplineRoad_C|GetSpline _splineroad))
  (Components|Timeline|SetPlayRate (Variables|Default|GetT_Move%20Object) (/ 1.0 (Variables|Default|GetTimeToEndPath)))
  (bind _movement_track (Timeline|T_Move%20Object PlayFromStart)
    (:Update
      (Transformation|SetActorLocationAndRotation (Spline|GetLocationatDistanceAlongSpline _spline (Math|Float|Lerp 0.0 (Spline|GetSplineLength _spline) _movement_track) "World") (Spline|GetRotationatDistanceAlongSpline _spline (Math|Float|Lerp 0.0 (Spline|GetSplineLength _spline) _movement_track) "World")))))

(event EventBeginPlay
  (CallFunction|FollowSpline))

(fn ConstructionScript
  (Components|StaticMesh|SetStaticMesh (Variables|Default|GetMeshBP) (Variables|Default|GetMeshToUse)))