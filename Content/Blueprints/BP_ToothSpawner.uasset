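; BP_ToothSpawner is an actor that spawns a single BP_Tooth at a randomly chosen location.
; On BeginPlay it calls the SpawnTooth event, which picks a random index into the ToothSpawn array and uses that entry as the spawn location.
; The chosen index is stored in CurrentIndex and printed on screen for debugging.
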(event Custom|SpawnTooth
  (bind _output_get (Variables|Default|SetCurrentIndex (Math|Random|RandomIntegerinRange 0 (- (Utilities|Array|Length (Variables|Default|GetToothSpawn)) 1))))
  (Game|SpawnActorfromClass "/Game/Blueprints/BP_Tooth.BP_Tooth_C" (Math|Transform|MakeTransform (Utilities|Array|Get(acopy) (Variables|Default|GetToothSpawn) _output_get) "0, 0, 0" "1.000000,1.000000,1.000000") "Undefined" "MultiplyWithRoot" 0 0)
  (Development|PrintString (Utilities|String|ToString(Integer) _output_get) true true "(R=1.000000,G=0.476340,B=0.000000,A=1.000000)" 6.0))

(event EventBeginPlay
  (CallFunction|SpawnTooth))

(event Collision|EventActorBeginOverlap
  (params (OtherActor :type Actor%20Object%20Reference)))

(event EventTick
  (params (DeltaSeconds :type Float%20%28single-precision%29)))

(fn ConstructionScript)