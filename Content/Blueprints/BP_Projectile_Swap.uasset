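; Projectile that swaps its caster's position with another BP_FirstPersonCharacter, with tornado Niagara effects.
; Overlapping a character swaps directly; Hit sphere-traces for the closest character to swap with.
; If that trace finds nothing, capsule traces step back from the projectile toward the caster to find a free teleport spot.
; After ExplosionDelay, Tick stops movement and tries a radius swap, destroying itself only when the trace finds nothing.
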(event EventBeginPlay)

(event Collision|EventHit
  (params (MyComp :type Primitive%20Component%20Object%20Reference) (Other :type Actor%20Object%20Reference) (OtherComp :type Primitive%20Component%20Object%20Reference) (bSelfMoved :type Boolean) (HitLocation :type Vector :default "0, 0, 0") (HitNormal :type Vector :default "0, 0, 0") (NormalImpulse :type Vector :default "0, 0, 0") (Hit :type Hit%20Result%20Structure%20%28by%20ref%29))
  (bind _returnvalue (Transformation|GetActorLocation))
  (bind _caster (Variables|Default|GetCaster))
  (bind _capsulecomponent (Variables|/Script/Engine.Character|GetCapsuleComponent _caster))
  (bind _returnvalue_2 (Components|Capsule|GetScaledCapsuleHalfHeight _capsulecomponent))
  (bind _returnvalue_3 (Components|Capsule|GetScaledCapsuleRadius _capsulecomponent))
  (CallFunction|FX (Variables|Default|GetCaster))
  (bind (_outhits _returnvalue_4) (Collision|MultiSphereTraceForObjects HitLocation HitLocation (Variables|Default|GetExplosionRadius) (Variables|Default|GetLayer) false 0 "ForDuration" true "(R=1.000000,G=0.000000,B=0.000000,A=1.000000)" "(R=0.000000,G=1.000000,B=0.000000,A=1.000000)" 1.0))
  (if _returnvalue_4
    (for _array_element _outhits
      (bind _asbp_first_person_character (Utilities|Casting|CastToBP_FirstPersonCharacter (.HitActor (Collision|BreakHitResult _array_element))))
      (if (== (Variables|Default|GetDistanceClosestPlayer) -1.0)
        (Variables|Default|SetDistanceClosestPlayer (Math|Vector|Distance(Vector) (Transformation|GetActorLocation _asbp_first_person_character) (Transformation|GetActorLocation)) :!label _label)
        (Variables|Default|SetClosestPlayer _asbp_first_person_character)
        (elif (< (Math|Vector|Distance(Vector) (Transformation|GetActorLocation _asbp_first_person_character) (Transformation|GetActorLocation)) (Variables|Default|GetDistanceClosestPlayer))
          (goto _label))))
    (Variables|Default|SetB_Pos (Transformation|GetActorLocation (Variables|Default|GetClosestPlayer)))
    (CallFunction|FX (Variables|Default|GetClosestPlayer))
    (Transformation|SetActorLocation (Variables|Default|GetClosestPlayer) (Transformation|GetActorLocation (Variables|Default|GetCaster)) false false)
    (Transformation|SetActorLocation (Variables|Default|GetCaster) (Variables|Default|GetB_Pos) false false)
    (Actor|DestroyActor)
    (else
      (bind _index (Utilities|FlowControl|ForLoopwithBreak 0 10 :!label _label_2)
        (:LoopBody
          (bind _returnvalue_5 (Collision|CapsuleTraceByChannel (+ (+ (* (Math|Vector|Normalize (- (Transformation|GetActorLocation (Variables|Default|GetCaster)) _returnvalue)) (* (* _returnvalue_3 2.0) (+ _index 1))) _returnvalue) (Math|Vector|MakeVector 0.0 0.0 _returnvalue_2)) (+ (+ (* (Math|Vector|Normalize (- (Transformation|GetActorLocation (Variables|Default|GetCaster)) _returnvalue)) (* (* _returnvalue_3 2.0) (+ _index 1))) _returnvalue) (Math|Vector|MakeVector 0.0 0.0 _returnvalue_2)) _returnvalue_3 _returnvalue_2 "TraceTypeQuery1" false 0 "ForDuration"))
          (if (not _returnvalue_5)
            (Transformation|SetActorLocation (Variables|Default|GetCaster) (+ (* (Math|Vector|Normalize (- (Transformation|GetActorLocation (Variables|Default|GetCaster)) _returnvalue)) (* (* _returnvalue_3 2.0) (+ _index 1))) _returnvalue) false false)
            (Niagara|SpawnSystematLocation "/Game/VFX/VFX/NS_Tornade.NS_Tornade" (Transformation|GetActorLocation) "0, 0, 0" "5.000000,5.000000,5.000000")
            (goto _label_2 Break)))
        (:Completed
          (Utilities|FlowControl|Delay 0.2)
          (Actor|DestroyActor))))))

(event EventTick
  (params (DeltaSeconds :type Float%20%28single-precision%29))
  (bind _returnvalue (Transformation|GetActorLocation))
  (bind _output_get (Variables|Default|SetcurrentDelay (+ DeltaSeconds (Variables|Default|GetcurrentDelay))))
  (if (>= _output_get (Variables|Default|GetExplosionDelay))
    (Variables|/Script/Engine.MovementComponent|SetVelocity (Variables|Default|GetProjectileMovement) "0, 0, 0")
    (bind (_outhits _returnvalue_2) (Collision|MultiSphereTraceForObjects _returnvalue _returnvalue (Variables|Default|GetExplosionRadius) (Variables|Default|GetLayer) false 0 "ForOneFrame" true "(R=1.000000,G=0.000000,B=0.000000,A=1.000000)" "(R=0.000000,G=1.000000,B=0.000000,A=1.000000)" 1.0))
    (if _returnvalue_2
      (for _array_element _outhits
        (bind _asbp_first_person_character (Utilities|Casting|CastToBP_FirstPersonCharacter (.HitActor (Collision|BreakHitResult _array_element))))
        (if (== (Variables|Default|GetDistanceClosestPlayer) -1.0)
          (Variables|Default|SetDistanceClosestPlayer 0.0 :!label _label)
          (Variables|Default|SetClosestPlayer _asbp_first_person_character)
          (elif (< (Math|Vector|Distance(Vector) (Transformation|GetActorLocation _asbp_first_person_character) (Transformation|GetActorLocation)) (Variables|Default|GetDistanceClosestPlayer))
            (goto _label))))
      (Variables|Default|SetB_Pos (Transformation|GetActorLocation (Variables|Default|GetClosestPlayer)))
      (Transformation|SetActorLocation (Variables|Default|GetClosestPlayer) (Transformation|GetActorLocation (Variables|Default|GetCaster)) false false)
      (Transformation|SetActorLocation (Variables|Default|GetCaster) (Variables|Default|GetB_Pos) false false)
      (else
        (Actor|DestroyActor)))))

(event Collision|EventActorBeginOverlap
  (params (OtherActor :type Actor%20Object%20Reference))
  (if (not (== OtherActor (Variables|Default|GetCaster)))
    (bind _asbp_first_person_character (Utilities|Casting|CastToBP_FirstPersonCharacter OtherActor))
    (CallFunction|FX (Variables|Default|GetCaster))
    (bind _output_get (Variables|Default|SetClosestPlayer _asbp_first_person_character))
    (Variables|Default|SetB_Pos (Transformation|GetActorLocation _output_get))
    (Niagara|SpawnSystematLocation "/Game/VFX/VFX/NS_Tornade.NS_Tornade" (Transformation|GetActorLocation _output_get) (Transformation|GetActorRotation _output_get))
    (Transformation|SetActorLocation _output_get (Transformation|GetActorLocation (Variables|Default|GetCaster)) false false)
    (Transformation|SetActorLocation (Variables|Default|GetCaster) (Variables|Default|GetB_Pos) false false)
    (Actor|DestroyActor)))

(fn ConstructionScript)

(fn FX
  (params (self3 :type Character%20Object%20Reference))
  (Niagara|SpawnSystematLocation "/Game/VFX/VFX/NS_Tornade.NS_Tornade" (- (Transformation|GetActorLocation self3) (Math|Vector|MakeVector 0.0 0.0 (Components|Capsule|GetScaledCapsuleHalfHeight (Variables|/Script/Engine.Character|GetCapsuleComponent self3)))) (Transformation|GetActorRotation self3) "5.000000,5.000000,5.000000"))