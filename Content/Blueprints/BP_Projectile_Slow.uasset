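; Projectile that slows player characters caught in its explosion, sparing the caster.
; It explodes on hit, on sphere overlap with anything but the caster, or once Tick accumulates the explosion delay.
; SlowExplosion runs a debug-drawn multi-sphere trace, spawns a Niagara effect, calls Slow on other first-person characters through SlowChara, then destroys the projectile.
; Older direct-cast and walk-speed slow logic remains unconnected.
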(event OnComponentBeginOverlap(Sphere)
  (params (OverlappedComponent :type Primitive%20Component%20Object%20Reference) (OtherActor :type Actor%20Object%20Reference) (OtherComp :type Primitive%20Component%20Object%20Reference) (OtherBodyIndex :type Integer) (bFromSweep :type Boolean) (SweepResult :type Hit%20Result%20Structure%20%28by%20ref%29))
  (bind _returnvalue (Transformation|GetActorLocation))
  (if (== OtherActor (Variables|Default|GetCaster))
    (Development|PrintString "Hello")
    (else
      (CallFunction|SlowExplosion _returnvalue _returnvalue))))

(event Custom|Slow%20Chara
  (params (Player%20Hit :type BP%20First%20Person%20Character%20Object%20Reference))
  (Default|Slow Player%20Hit))

(event EventBeginPlay)

(event Collision|EventActorBeginOverlap
  (params (OtherActor :type Actor%20Object%20Reference)))

(event Collision|EventHit
  (params (MyComp :type Primitive%20Component%20Object%20Reference) (Other :type Actor%20Object%20Reference) (OtherComp :type Primitive%20Component%20Object%20Reference) (bSelfMoved :type Boolean) (HitLocation :type Vector :default "0, 0, 0") (HitNormal :type Vector :default "0, 0, 0") (NormalImpulse :type Vector :default "0, 0, 0") (Hit :type Hit%20Result%20Structure%20%28by%20ref%29))
  (CallFunction|SlowExplosion HitLocation HitLocation))

(event EventTick
  (params (DeltaSeconds :type Float%20%28single-precision%29))
  (bind _returnvalue (Transformation|GetActorLocation))
  (bind _output_get (Variables|Default|SetcurrentDelay (+ DeltaSeconds (Variables|Default|GetcurrentDelay))))
  (if (>= _output_get (Variables|Default|GetExplosionDelay))
    (Variables|/Script/Engine.MovementComponent|SetVelocity (Variables|Default|GetProjectileMovement) "0, 0, 0")
    (CallFunction|SlowExplosion _returnvalue _returnvalue)))

(fn ConstructionScript)

(fn SlowExplosion
  (params (End :type Vector) (Start :type Vector))
  (bind _returnvalue (Transformation|GetActorTransform))
  (bind (_outhits _returnvalue_2) (Collision|MultiSphereTraceForObjects Start End (Variables|Default|GetExplosionRadius) (Variables|Default|GetLayer) false 0 "ForDuration" true "(R=1.000000,G=0.000000,B=0.000000,A=1.000000)" "(R=0.000000,G=1.000000,B=0.000000,A=1.000000)" 1.0))
  (Niagara|SpawnSystematLocation "/Game/VFX/VFX/NS_slow_explode.NS_slow_explode" (.location _returnvalue) (.rotation _returnvalue))
  (if _returnvalue_2
    (for _array_element _outhits
      (bind _asbp_first_person_character (Utilities|Casting|CastToBP_FirstPersonCharacter (.HitActor (Collision|BreakHitResult _array_element))))
      (if (not (== _asbp_first_person_character (Variables|Default|GetCaster)))
        (CallFunction|SlowChara _asbp_first_person_character))))
  (Actor|DestroyActor))